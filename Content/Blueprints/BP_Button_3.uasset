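; Interactable push button that animates when used and then signals a door to open.
; On BeginPlay it binds to the AC3DInteractive component's start-interact event to trigger the press.
; The PressButtom timeline slides the static mesh along relative X, then fires OpenDoor when finished.
; Label-cycling logic over ButtonText is left disconnected and never runs.
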(event Custom|EventPressButtom
  (bind _staticmesh (Variables|Default|GetStaticMesh))
  (bind _relativelocation (Variables|/Script/Engine.SceneComponent|GetRelativeLocation _staticmesh))
  (bind _pressbuttom (Timeline|PressButtom PlayFromStart)
    (:Update
      (Transformation|SetRelativeLocation (Variables|Default|GetStaticMesh) (Math|Vector|MakeVector (* 20 _pressbuttom) (.y _relativelocation) (.z _relativelocation)) false false))
    (:Finished
      (Default|CallOpenDoor))))

(event EventBeginPlay
  (|CallParentFunction)
  (Protected|Bind|BindingEvents))

(fn ConstructionScript)

(fn BindingEvents
  (EventDispatchers|BindEventtoOnStartInteract (Variables|Default|GetAC_3D_Interactive) (EventDispatchers|CreateEvent :!event BindonStartInteract)))

(fn BindonStartInteract
  ;[1 1 1] Изменение надписи кнопки
  (Utilities|FlowControl|Sequence
    (:then_1
      (CallFunction|EventPressButtom))))