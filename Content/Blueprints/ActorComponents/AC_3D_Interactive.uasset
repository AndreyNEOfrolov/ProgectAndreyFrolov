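; Actor component for 3D interactive objects that raises interact and touch events and shows a floating context hint.
; StartTouch fires its event and spawns a single BP_ContextHint at the owner plus TextLocation, while EndTouch fires its event and destroys it.
; Each Tick turns the hint toward the player pawn and repositions it at the stored target mesh's location plus that offset.
; StartInteract only fires its event; the stop-interact call is unconnected.
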(event EventTick
  (params (DeltaSeconds :type Float%20%28single-precision%29))
  (bind _bp_textrender (Variables|Private|GetBP_TextRender))
  (bind _statick_mesh (Variables|Default|GetStatick%20Mesh))
  (bind _textlocation (Variables|Config|GetTextLocation))
  (bind _returnvalue (Transformation|GetWorldLocation _statick_mesh))
  ;[1 1 1] Вращение подсказки к павну и вертикальное позиционирование
  (Utilities|IsValid _bp_textrender
    (:Is%20Valid
      (Transformation|SetActorRelativeRotation (Variables|Private|GetBP_TextRender) (Math|Rotator|FindLookatRotation (Transformation|GetWorldLocation (Variables|/Game/Blueprints/BaseObjects/BP_ContextHint.BP_ContextHint_C|GetTextRender _bp_textrender)) (Transformation|GetActorLocation (Game|Player|GetPlayerPawn 0))))
      (Transformation|SetActorRelativeLocation (Variables|Private|GetBP_TextRender) (Math|Vector|MakeVector (+ (.x _textlocation) (.x _returnvalue)) (+ (.y _textlocation) (.y _returnvalue)) (+ (.z _returnvalue) (.z _textlocation)))))))

(fn StartInteract
  (Default|CallOnStartInteract))

(fn StartTouch
  (Default|CallOnTouch)
  (Private|SpawnTextRender))

(fn EndTouch
  (Default|CallOnEndTouch)
  (bind _bp_textrender (Variables|Private|GetBP_TextRender)
    (:then
      (Actor|DestroyActor _bp_textrender))
    (:else)))

(fn SpawnTextRender
  (bind _returnvalue (Components|GetOwner))
  (bind _textlocation (Variables|Config|GetTextLocation))
  (bind _returnvalue_2 (Transformation|GetActorTransform _returnvalue))
  ;[1 1 1] Спавн контекстной подсказки
  (Variables|Private|GetBP_TextRender
    (:then)
    (:else
      (bind _returnvalue_3 (Game|SpawnActorfromClass "/Game/Blueprints/BaseObjects/BP_ContextHint.BP_ContextHint_C" (Math|Transform|MakeTransform (Math|Vector|MakeVector (+ (.x (.location _returnvalue_2)) (.x _textlocation)) (+ (.y (.location _returnvalue_2)) (.y _textlocation)) (+ (.z (.location _returnvalue_2)) (.z _textlocation))) (.rotation _returnvalue_2) "1,1,1") "Undefined" _returnvalue 0))
      (Variables|Private|SetBP_TextRender _returnvalue_3))))

(fn SetFirstTarget
  (params (StatickMesh :type Static%20Mesh%20Component%20Object%20Reference))
  (Variables|Default|SetStatick%20Mesh StatickMesh))

(fn GetFirstTarget
  (return (Variables|Default|GetStatick%20Mesh)))