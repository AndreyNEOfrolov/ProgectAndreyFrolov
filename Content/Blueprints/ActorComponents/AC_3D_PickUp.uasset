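; Actor component for 3D pick-up items that switches the owning actor between held and dropped states.
; Grab disables physics and collision on the target from the parent class's GetFirstTarget, leaving attachment to code outside this component.
; Drop re-enables both and detaches the owner, keeping its world transform.
; Both functions fire the OnDrop dispatcher, so listeners receive the same event for grabbing and dropping.
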(event EventBeginPlay
  (|CallParentFunction) ; This node is disabled and will not be called.\nDrag off pins to build functionality.
)

(event EventTick
  (params (DeltaSeconds :type Float%20%28single-precision%29)))

(fn Drop
  (bind _statick_mesh (CallFunction|GetFirstTarget))
  ;[1 1 1] Отпускание предмета из рук
  (Default|CallOnDrop)
  (Physics|SetSimulatePhysics _statick_mesh true)
  (Collision|SetCollisionEnabled _statick_mesh "QueryAndPhysics")
  (Transformation|DetachFromActor (Components|GetOwner) "KeepWorld" "KeepWorld" "KeepWorld"))

(fn Grab
  (bind _statick_mesh (CallFunction|GetFirstTarget))
  ;[1 1 1] Отключение физики и коллизи обьекта в руках и вызов диспатчера
  (Default|CallOnDrop)
  (Physics|SetSimulatePhysics _statick_mesh false)
  (Collision|SetCollisionEnabled _statick_mesh "NoCollision"))

(fn GetFirstTarget
  (return (|CallParentFunction)))