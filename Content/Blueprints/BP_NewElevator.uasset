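; BP_NewElevator is an elevator actor that moves its Kube component between a lowered and a raised position.
; On BeginPlay it caches two child-actor BP_ElevateButtons and binds an event to each one's ED2 dispatcher.
; UpDown flips a boolean to alternate between UpElevate and DownElevate, whose separate timelines lerp Kube's relative height.
; A FirstPersonCharacter dispatcher binding is left disconnected.
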(event Custom|ED1_Event_0
  (params (NewParam :type Float%20%28single-precision%29) (NewParam1 :type Float%20%28single-precision%29)))

(event Custom|DownElevate
  (bind _newtrack_0 (Timeline|Timeline_0 PlayFromStart)
    (:Update
      (Transformation|SetRelativeLocation (Variables|Default|GetKube) (Math|Vector|Lerp(Vector) "0, 0,290.000000" "0, 0, 0" _newtrack_0) false false))))

(event Custom|UpElevate
  (bind _float (Timeline|MoveElevate PlayFromStart)
    (:Update
      (Transformation|SetRelativeLocation (Variables|Default|GetKube) (Math|Vector|Lerp(Vector) "0, 0, 0" "0, 0,290.000000" _float) false false))))

(event EventBeginPlay
  (CallFunction|InitVarriable)
  (CallFunction|BindingEvents))

(fn ConstructionScript)

(fn InitVarriable
  (Utilities|FlowControl|Sequence
    (:then_0
      (bind _asbp_elevate_button (Utilities|Casting|CastToBP_ElevateButton (Variables|/Script/Engine.ChildActorComponent|GetChildActor (Variables|Default|GetChildActorButton))))
      (Variables|Default|SetAs%20BP%20Elevate%20Button _asbp_elevate_button))
    (:then_1
      (bind _asbp_elevate_button_2 (Utilities|Casting|CastToBP_ElevateButton (Variables|/Script/Engine.ChildActorComponent|GetChildActor (Variables|Default|GetChildActorButton1))))
      (Variables|Default|SetAs%20BP%20Elevate%20Button_0 _asbp_elevate_button_2))))

(fn BindingEvents
  (EventDispatchers|BindEventtoED2 (Variables|Default|GetAs%20BP%20Elevate%20Button) (EventDispatchers|CreateEvent :!event Up/Down)))

(fn Up/Down
  (if (Variables|Default|GetNewVar_0)
    (CallFunction|UpElevate)
    (Variables|Default|SetNewVar_0 false)
    (else
      (CallFunction|DownElevate)
      (Variables|Default|SetNewVar_0 true))))