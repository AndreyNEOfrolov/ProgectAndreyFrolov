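; BP_Button_2 is an interactive 3D button that cycles its displayed label and animates a press when used.
; On BeginPlay it runs parent logic and binds to the start-interact event of its AC3DInteractive component.
; Each interaction sets the text render to the next ButtonText entry, wrapping at the end of the array.
; It also restarts the PressButtom timeline, which offsets the static mesh along its relative X axis.
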(event Custom|EventPressButtom
  (bind _staticmesh (Variables|Default|GetStaticMesh))
  (bind _relativelocation (Variables|/Script/Engine.SceneComponent|GetRelativeLocation _staticmesh))
  (bind _pressbuttom (Timeline|PressButtom PlayFromStart)
    (:Update
      (Transformation|SetRelativeLocation (Variables|Default|GetStaticMesh) (Math|Vector|MakeVector (* 20 _pressbuttom) (.y _relativelocation) (.z _relativelocation)) false false))))

(event EventBeginPlay
  (|CallParentFunction)
  (Protected|Bind|BindingEvents))

(fn ConstructionScript)

(fn BindingEvents
  (EventDispatchers|BindEventtoOnStartInteract (Variables|Default|GetAC_3D_Interactive) (EventDispatchers|CreateEvent :!event BindonStartInteract)))

(fn BindonStartInteract
  (bind _buttontext (Variables|Private|GetButtonText))
  ;[1 1 1] Изменение надписи кнопки
  (Utilities|FlowControl|Sequence
    (:then_0
      (Rendering|Components|TextRender|SetText (Variables|Default|GetTextRender) (Utilities|Array|Get(acopy) _buttontext (Variables|Private|GetCurrentText)))
      (Math|Integer|IncrementInt (Variables|Private|GetCurrentText)
        (:%20%20
          (if (== (Variables|Private|GetCurrentText) (Utilities|Array|Length _buttontext))
            (Variables|Private|SetCurrentText 0)))))
    (:then_1
      (CallFunction|EventPressButtom))))