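; Door actor that slides its Cube along local Z between its origin and 420 units below it.
; On BeginPlay it caches the BP_Button_3 from its child actor and binds to that button's OpenDoor event.
; OpenClose alternates between the Up and Down timelines via a boolean.
; Down, which returns the cube to origin, disables its collision without re-enabling it and prints the position each update.
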(event Custom|Up
  ;[1 1 1] Анимация открывания двери.
  (bind _float (Timeline|OpenDoor PlayFromStart)
    (:Update
      (Transformation|SetRelativeLocation (Variables|Default|GetCube) (Math|Vector|Lerp(Vector) "0, 0, 0" "0, 0,-420.000000" _float) false false))))

(event Custom|Down
  ;[1 1 1] Анимация открывания двери.
  (Collision|SetCollisionEnabled (Variables|Default|GetCube) "NoCollision")
  (bind _float (Timeline|Timeline_0 PlayFromStart)
    (:Update
      (Development|PrintString (Utilities|String|ToString(Vector) (Math|Vector|Lerp(Vector) "0, 0,-420.000000" "0, 0, 0" _float)))
      (Transformation|SetRelativeLocation (Variables|Default|GetCube) (Math|Vector|Lerp(Vector) "0, 0,-420.000000" "0, 0, 0" _float) false false))))

(event EventBeginPlay
  ;[1 1 1] Анимация открывания двери.
  (CallFunction|IntVAR)
  (CallFunction|BindEvents))

(fn ConstructionScript)

(fn IntVAR
  (bind _asbp_button_3 (Utilities|Casting|CastToBP_Button_3 (Variables|/Script/Engine.ChildActorComponent|GetChildActor (Variables|Default|GetChildActor))))
  (Variables|Default|SetButton3 _asbp_button_3))

(fn BindEvents
  (EventDispatchers|BindEventtoOpenDoor (Variables|Default|GetButton3) (EventDispatchers|CreateEvent :!event Open/Close)))

(fn Open/Close
  (if (Variables|Default|GetVarUpDown)
    (CallFunction|Up)
    (Variables|Default|SetVarUpDown false)
    (else
      (CallFunction|Down)
      (Variables|Default|SetVarUpDown true))))