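; BP_ElevateButton is an interactive button, named for an elevator, that animates a press when the player interacts with it.
; On BeginPlay it binds to the AC3DInteractive component's start-interact event, and the construction script sets that component's text location.
; Interaction plays a timeline that slides the mesh along local X, then calls the CallED2 dispatcher when finished.
; Logic for cycling the button's label text is present but disconnected.
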(event Custom|EventPressButtom
  (bind _staticmesh (Variables|Default|GetStaticMesh))
  (bind _relativelocation (Variables|/Script/Engine.SceneComponent|GetRelativeLocation _staticmesh))
  (bind _pressbuttom (Timeline|PressButtom PlayFromStart)
    (:Update
      (Transformation|SetRelativeLocation (Variables|Default|GetStaticMesh) (Math|Vector|MakeVector (* -20 _pressbuttom) (.y _relativelocation) (.z _relativelocation)) false false))
    (:Finished
      (Default|CallED2))))

(event EventBeginPlay
  (|CallParentFunction)
  (Protected|Bind|BindingEvents))

(fn ConstructionScript
  (Variables|/Game/Blueprints/ActorComponents/AC_3D_Interactive.AC_3D_Interactive_C|SetTextLocation (Variables|Default|GetAC_3D_Interactive) (Variables|Default|GetButton%20Location)))

(fn BindingEvents
  (EventDispatchers|BindEventtoOnStartInteract (Variables|Default|GetAC_3D_Interactive) (EventDispatchers|CreateEvent :!event BindonStartInteract)))

(fn BindonStartInteract
  ;[1 1 1] Изменение надписи кнопки
  (Utilities|FlowControl|Sequence
    (:then_1
      (CallFunction|EventPressButtom))))