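; Box platform actor that takes the object a FirstPersonCharacter is carrying and seats it in place when overlapped while empty.
; A timeline lerps the grabbed actor's location and rotation to the Scene component, preserving its scale.
; It then attaches the actor, makes the character drop it, and, through its AC_3D_PickUp component, disables physics and flags the platform occupied.
; The flag clears when that actor leaves the Box component.
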(event OnComponentEndOverlap(Box)
  (params (OverlappedComponent :type Primitive%20Component%20Object%20Reference) (OtherActor :type Actor%20Object%20Reference) (OtherComp :type Primitive%20Component%20Object%20Reference) (OtherBodyIndex :type Integer))
  (if (== OtherActor (Variables|Default|GetCurrent%20Pick%20Up%20Actor))
    (Variables|Default|SetBoxOnPlatform false)))

(event Collision|EventActorBeginOverlap
  (params (OtherActor :type Actor%20Object%20Reference))
  (if (not (Variables|Default|GetBoxOnPlatform))
    (bind _asfirst_person_character (Utilities|Casting|CastToFirstPersonCharacter OtherActor))
    (Variables|Default|SetBP_Character _asfirst_person_character)
    (Utilities|IsValid (Default|GetGrabbedActor _asfirst_person_character)
      (:Is%20Valid
        (bind _output_get (Variables|Default|SetCurrent%20Pick%20Up%20Actor (Default|GetGrabbedActor _asfirst_person_character)))
        (Variables|Default|SetInitialTransform (Transformation|GetActorTransform _output_get))
        (bind _alpha (Timeline|Timeline_0 PlayFromStart)
          (:Update
            (Transformation|SetActorTransform (Variables|Default|GetCurrent%20Pick%20Up%20Actor) (Math|Transform|MakeTransform (.Location (Math|Transform|BreakTransform (Math|Transform|Lerp(Transform) (Variables|Default|GetInitialTransform) (Transformation|GetWorldTransform (Variables|Default|GetScene)) _alpha))) (.Rotation (Math|Transform|BreakTransform (Math|Transform|Lerp(Transform) (Variables|Default|GetInitialTransform) (Transformation|GetWorldTransform (Variables|Default|GetScene)) _alpha))) (.scale (Variables|Default|GetInitialTransform)))))
          (:Finished
            (Transformation|SetWorldScale3D (Variables|Default|GetScene) (.scale (Variables|Default|GetInitialTransform)))
            (Transformation|AttachComponentToComponent (Variables|Default|GetCurrent%20Pick%20Up%20Actor) (Variables|Default|GetScene) "None" "SnapToTarget" "SnapToTarget" "SnapToTarget" true)
            (Default|DropPickUpComponent (Variables|Default|GetBP_Character))
            (Utilities|IsValid (Actor|GetComponentbyClass (Variables|Default|GetCurrent%20Pick%20Up%20Actor) "/Game/Blueprints/ActorComponents/AC_3D_PickUp.AC_3D_PickUp_C")
              (:Is%20Valid
                (Physics|SetSimulatePhysics (Default|GetFirstTarget (Actor|GetComponentbyClass (Variables|Default|GetCurrent%20Pick%20Up%20Actor) "/Game/Blueprints/ActorComponents/AC_3D_PickUp.AC_3D_PickUp_C")) false)
                (Variables|Default|SetBoxOnPlatform true)))))))))

(fn ConstructionScript)